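; Interaction-state actor that fills the player's MainCanvas widget with random floating sentences from MyGameManager's data.
; A Tick timer or the Q key spawns each sentence.
; A reverse loop ages sentences through a font-material "Timer" parameter, removing expired ones and recycling their grid slots.
; Key 1 plays a timeline that hides the QR code, then calls StateDone on MyFSMManager to end the state.
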(event EventBeginPlay
  (Input|EnableInput (Game|GetPlayerController 0))
  (Development|PrintText "Interaction")
  (bind _asmy_character (Utilities|Casting|CastToMyCharacter (Game|GetPlayerCharacter 0)))
  (Variables|Default|Setwidget (Variables|/Game/Blueprints/MyCharacter.MyCharacter_C|Getwidget _asmy_character)))

(event Collision|EventActorBeginOverlap
  (params (OtherActor :type Actor%20Object%20Reference)))

(event EventTick
  (params (DeltaSeconds :type Float%20%28single-precision%29))
  (bind _output_get (Variables|Default|Settimer (+ DeltaSeconds (Variables|Default|Gettimer))))
  (if (> _output_get 0.5)
    (Variables|Default|Settimer 0.0)
    (bind _asmain_canvas (Utilities|Casting|CastToMainCanvas (Variables|Default|Getwidget)))
    (bind _returnvalue (Actor|GetActorOfClass "/Game/Blueprints/MyGameManager.MyGameManager_C"))
    (Default|SpawnText _asmain_canvas (Utilities|Array|Get(acopy) (Variables|/Script/HuaweiWall.DataManager|GetSentences (Variables|/Game/Blueprints/MyGameManager.MyGameManager_C|GetdataManager _returnvalue)) (Math|Random|RandomInteger 9))))
  (bind _asmain_canvas_2 (Utilities|Casting|CastToMainCanvas (Variables|Default|Getwidget)))
  (if (> (Utilities|Array|Length (Variables|/Game/Widget/MainCanvas.MainCanvas_C|GetTimer _asmain_canvas_2)) 0)
    (for _index (range 0 (- (Utilities|Array|Length (Variables|/Game/Widget/MainCanvas.MainCanvas_C|GetTimer _asmain_canvas_2)) 1))
      (if (<= (Utilities|Array|Get(acopy) (Variables|/Game/Widget/MainCanvas.MainCanvas_C|GetTimer _asmain_canvas_2) (- (- (Utilities|Array|Length (Variables|/Game/Widget/MainCanvas.MainCanvas_C|GetTimer _asmain_canvas_2)) 1) _index)) 8.0)
        (Utilities|Array|SetArrayElem (Variables|/Game/Widget/MainCanvas.MainCanvas_C|GetTimer _asmain_canvas_2) (- (- (Utilities|Array|Length (Variables|/Game/Widget/MainCanvas.MainCanvas_C|GetTimer _asmain_canvas_2)) 1) _index) (+ (Utilities|Array|Get(acopy) (Variables|/Game/Widget/MainCanvas.MainCanvas_C|GetTimer _asmain_canvas_2) (- (- (Utilities|Array|Length (Variables|/Game/Widget/MainCanvas.MainCanvas_C|GetTimer _asmain_canvas_2)) 1) _index)) DeltaSeconds))
        (bind _returnvalue_2 (Class|TextBlock|GetDynamicFontMaterial (Utilities|Array|Get(acopy) (Variables|/Game/Widget/MainCanvas.MainCanvas_C|GetSentenceArray _asmain_canvas_2) (- (- (Utilities|Array|Length (Variables|/Game/Widget/MainCanvas.MainCanvas_C|GetTimer _asmain_canvas_2)) 1) _index))))
        (Rendering|Material|SetScalarParameterValue _returnvalue_2 "Timer" (+ (Utilities|Array|Get(acopy) (Variables|/Game/Widget/MainCanvas.MainCanvas_C|GetTimer _asmain_canvas_2) (- (- (Utilities|Array|Length (Variables|/Game/Widget/MainCanvas.MainCanvas_C|GetTimer _asmain_canvas_2)) 1) _index)) DeltaSeconds) :!class /Script/Engine.MaterialInstanceDynamic)
        (else
          (Widget|RemovefromParent (Utilities|Array|Get(acopy) (Variables|/Game/Widget/MainCanvas.MainCanvas_C|GetSentenceArray _asmain_canvas_2) (- (- (Utilities|Array|Length (Variables|/Game/Widget/MainCanvas.MainCanvas_C|GetTimer _asmain_canvas_2)) 1) _index)))
          (Utilities|Array|RemoveIndex (Variables|/Game/Widget/MainCanvas.MainCanvas_C|GetSentenceArray _asmain_canvas_2) (- (- (Utilities|Array|Length (Variables|/Game/Widget/MainCanvas.MainCanvas_C|GetTimer _asmain_canvas_2)) 1) _index))
          (Utilities|Array|RemoveIndex (Variables|/Game/Widget/MainCanvas.MainCanvas_C|GetTimer _asmain_canvas_2) (- (- (Utilities|Array|Length (Variables|/Game/Widget/MainCanvas.MainCanvas_C|GetTimer _asmain_canvas_2)) 1) _index))
          (Variables|/Game/Widget/MainCanvas.MainCanvas_C|SetAvilableGridSize _asmain_canvas_2 (+ (Variables|/Game/Widget/MainCanvas.MainCanvas_C|GetAvilableGridSize _asmain_canvas_2) 1))
          (Utilities|Array|Add (Variables|/Game/Widget/MainCanvas.MainCanvas_C|GetGridIndexArray _asmain_canvas_2) (Utilities|Array|Get(acopy) (Variables|/Game/Widget/MainCanvas.MainCanvas_C|GetUsedGridIndexArray _asmain_canvas_2)))
          (Utilities|Array|RemoveIndex (Variables|/Game/Widget/MainCanvas.MainCanvas_C|GetUsedGridIndexArray _asmain_canvas_2)))))))

(event Input|KeyboardEvents|Q
  (params (Key :type Key%20Structure :default "None"))
  (:Pressed
    (bind _asmain_canvas (Utilities|Casting|CastToMainCanvas (Variables|Default|Getwidget)))
    (bind _returnvalue (Actor|GetActorOfClass "/Game/Blueprints/MyGameManager.MyGameManager_C"))
    (Default|SpawnText _asmain_canvas (Utilities|Array|Get(acopy) (Variables|/Script/HuaweiWall.DataManager|GetSentences (Variables|/Game/Blueprints/MyGameManager.MyGameManager_C|GetdataManager _returnvalue)) (Math|Random|RandomInteger 9)))
    (bind _asmain_canvas_2 (Utilities|Casting|CastToMainCanvas (Variables|Default|Getwidget)))
    (if (> (Utilities|Array|Length (Variables|/Game/Widget/MainCanvas.MainCanvas_C|GetTimer _asmain_canvas_2)) 0)
      (for _index (range 0 (- (Utilities|Array|Length (Variables|/Game/Widget/MainCanvas.MainCanvas_C|GetTimer _asmain_canvas_2)) 1))
        (if (<= (Utilities|Array|Get(acopy) (Variables|/Game/Widget/MainCanvas.MainCanvas_C|GetTimer _asmain_canvas_2) (- (- (Utilities|Array|Length (Variables|/Game/Widget/MainCanvas.MainCanvas_C|GetTimer _asmain_canvas_2)) 1) _index)) 8.0)
          (Utilities|Array|SetArrayElem (Variables|/Game/Widget/MainCanvas.MainCanvas_C|GetTimer _asmain_canvas_2) (- (- (Utilities|Array|Length (Variables|/Game/Widget/MainCanvas.MainCanvas_C|GetTimer _asmain_canvas_2)) 1) _index) (+ (Utilities|Array|Get(acopy) (Variables|/Game/Widget/MainCanvas.MainCanvas_C|GetTimer _asmain_canvas_2) (- (- (Utilities|Array|Length (Variables|/Game/Widget/MainCanvas.MainCanvas_C|GetTimer _asmain_canvas_2)) 1) _index)) (stale EventTick DeltaSeconds)))
          (bind _returnvalue_2 (Class|TextBlock|GetDynamicFontMaterial (Utilities|Array|Get(acopy) (Variables|/Game/Widget/MainCanvas.MainCanvas_C|GetSentenceArray _asmain_canvas_2) (- (- (Utilities|Array|Length (Variables|/Game/Widget/MainCanvas.MainCanvas_C|GetTimer _asmain_canvas_2)) 1) _index))))
          (Rendering|Material|SetScalarParameterValue _returnvalue_2 "Timer" (+ (Utilities|Array|Get(acopy) (Variables|/Game/Widget/MainCanvas.MainCanvas_C|GetTimer _asmain_canvas_2) (- (- (Utilities|Array|Length (Variables|/Game/Widget/MainCanvas.MainCanvas_C|GetTimer _asmain_canvas_2)) 1) _index)) (stale EventTick DeltaSeconds)) :!class /Script/Engine.MaterialInstanceDynamic)
          (else
            (Widget|RemovefromParent (Utilities|Array|Get(acopy) (Variables|/Game/Widget/MainCanvas.MainCanvas_C|GetSentenceArray _asmain_canvas_2) (- (- (Utilities|Array|Length (Variables|/Game/Widget/MainCanvas.MainCanvas_C|GetTimer _asmain_canvas_2)) 1) _index)))
            (Utilities|Array|RemoveIndex (Variables|/Game/Widget/MainCanvas.MainCanvas_C|GetSentenceArray _asmain_canvas_2) (- (- (Utilities|Array|Length (Variables|/Game/Widget/MainCanvas.MainCanvas_C|GetTimer _asmain_canvas_2)) 1) _index))
            (Utilities|Array|RemoveIndex (Variables|/Game/Widget/MainCanvas.MainCanvas_C|GetTimer _asmain_canvas_2) (- (- (Utilities|Array|Length (Variables|/Game/Widget/MainCanvas.MainCanvas_C|GetTimer _asmain_canvas_2)) 1) _index))
            (Variables|/Game/Widget/MainCanvas.MainCanvas_C|SetAvilableGridSize _asmain_canvas_2 (+ (Variables|/Game/Widget/MainCanvas.MainCanvas_C|GetAvilableGridSize _asmain_canvas_2) 1))
            (Utilities|Array|Add (Variables|/Game/Widget/MainCanvas.MainCanvas_C|GetGridIndexArray _asmain_canvas_2) (Utilities|Array|Get(acopy) (Variables|/Game/Widget/MainCanvas.MainCanvas_C|GetUsedGridIndexArray _asmain_canvas_2)))
            (Utilities|Array|RemoveIndex (Variables|/Game/Widget/MainCanvas.MainCanvas_C|GetUsedGridIndexArray _asmain_canvas_2))))))))

(event Input|KeyboardEvents|1
  (params (Key :type Key%20Structure :default "None"))
  (:Pressed
    (bind _asmain_canvas (Utilities|Casting|CastToMainCanvas (Variables|Default|Getwidget)))
    (bind _新建轨道_0 (Timeline|时间轴 PlayFromStart)
      (:Update
        (Default|HideQrCode _asmain_canvas _新建轨道_0))
      (:Finished
        (bind _returnvalue (Actor|GetActorOfClass "/Game/Blueprints/MyFSMManager.MyFSMManager_C"))
        (Default|StateDone _returnvalue)))))

(fn ConstructionScript)

(fn FadeText)