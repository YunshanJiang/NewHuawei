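; Game manager actor that runs startup setup for configuration, window size, API links and the main UI.
; On BeginPlay it loads data through DataManager, then copies the window dimensions to WindowManager and the GetData and PostData endpoints to APIManager.
; After a brief delay it reaches the player character's MainCanvas widget and initializes its sentence images from the loaded sentences.
; An always-on-top window call is present but unconnected.
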(event EventBeginPlay
  (bind _apimanager (Variables|Default|GetAPIManager))
  (bind _datamanager (Variables|Default|GetdataManager))
  (bind _windowmanager (Variables|Default|GetWindowManager))
  (Class|DataManager|LoadData _datamanager)
  (Variables|/Script/HuaweiWall.WindowManager|SetWindowWidth _windowmanager (Variables|/Script/HuaweiWall.DataManager|GetWindowWidth _datamanager))
  (Variables|/Script/HuaweiWall.WindowManager|SetWindowHeight _windowmanager (Variables|/Script/HuaweiWall.DataManager|GetWindowHeight _datamanager))
  (Variables|/Script/HuaweiWall.APIManager|SetgetDataLink _apimanager (Class|DataManager|GetAPI _datamanager "GetData"))
  (Variables|/Script/HuaweiWall.APIManager|SetpostDataLink _apimanager (Class|DataManager|GetAPI _datamanager "PostData"))
  (Utilities|FlowControl|Delay 0.005)
  (bind _asmy_character (Utilities|Casting|CastToMyCharacter (Game|GetPlayerCharacter 0)))
  (bind _asmain_canvas (Utilities|Casting|CastToMainCanvas (Variables|/Game/Blueprints/MyCharacter.MyCharacter_C|Getwidget _asmy_character)))
  (Default|InitSentenceImg _asmain_canvas (Variables|/Script/HuaweiWall.DataManager|GetSentences _datamanager)))

(event Collision|EventActorBeginOverlap
  (params (OtherActor :type Actor%20Object%20Reference)))

(event EventTick
  (params (DeltaSeconds :type Float%20%28single-precision%29)))

(fn ConstructionScript)