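; MyIntroState is the intro state actor that resets the scene and waits for the 1 key.
; On BeginPlay, Init resets the MainCanvas widget, Aurora and AuroraExplosion materials, and cine camera rotation.
; Pressing 1 plays a timeline that drives the QR code position, then calls StateDone on MyFSMManager.
; An unconnected branch that would load MyDataManager sentences into the canvas never runs.
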(event EventBeginPlay
  (Input|EnableInput (Game|GetPlayerController 0))
  (CallFunction|Init))

(event Collision|EventActorBeginOverlap
  (params (OtherActor :type Actor%20Object%20Reference)))

(event EventTick
  (params (DeltaSeconds :type Float%20%28single-precision%29)))

(event Input|KeyboardEvents|1
  (params (Key :type Key%20Structure :default "None"))
  (:Pressed
    (bind _asmy_character (Utilities|Casting|CastToMyCharacter (Game|GetPlayerCharacter 0)))
    (bind _新建轨道_0 (Timeline|时间轴 Play)
      (:Update
        (bind _asmain_canvas (Utilities|Casting|CastToMainCanvas (Variables|/Game/Blueprints/MyCharacter.MyCharacter_C|Getwidget _asmy_character)))
        (Default|SetQRCodePos _asmain_canvas _新建轨道_0))
      (:Finished
        (bind _returnvalue (Actor|GetActorOfClass "/Game/Blueprints/MyFSMManager.MyFSMManager_C"))
        (Default|StateDone _returnvalue)))))

(fn ConstructionScript)

(fn Init
  (bind _asmy_character (Utilities|Casting|CastToMyCharacter (Game|GetPlayerCharacter 0)))
  (bind _asmain_canvas (Utilities|Casting|CastToMainCanvas (Variables|/Game/Blueprints/MyCharacter.MyCharacter_C|Getwidget _asmy_character)))
  (Default|HideQrCode _asmain_canvas 1.0)
  (Default|SetQRCodePos _asmain_canvas 0.0)
  (bind _returnvalue (Actor|GetActorOfClass "/Game/Blueprints/Aurora.Aurora_C"))
  (bind _returnvalue_2 (Actor|GetActorOfClass "/Game/Blueprints/AuroraExplosion.AuroraExplosion_C"))
  (Rendering|Material|SetScalarParameterValue (Variables|/Game/Blueprints/Aurora.Aurora_C|GetmyMaterial _returnvalue) "Hide" 0.0 :!class /Script/Engine.MaterialInstanceDynamic)
  (Rendering|Material|SetScalarParameterValue (Variables|/Game/Blueprints/AuroraExplosion.AuroraExplosion_C|GetMyMaterial _returnvalue_2) "Opacity" 0.0 :!class /Script/Engine.MaterialInstanceDynamic)
  (Rendering|Material|SetScalarParameterValue (Variables|/Game/Blueprints/Aurora.Aurora_C|GetmyMaterial _returnvalue) "Opacity" 0.0 :!class /Script/Engine.MaterialInstanceDynamic)
  (Default|EndingTextShow _asmain_canvas 0.0)
  (Default|ResetSentenceImgUI _asmain_canvas)
  (bind _returnvalue_3 (Actor|GetActorOfClass "/Script/CinematicCamera.CineCameraActor"))
  (Transformation|SetRelativeRotation (Class|CineCameraActor|GetCineCameraComponent _returnvalue_3) (Math|Rotator|MakeRotator 0.0 0.0 0.0) false false)
  (Class|Image|SetOpacity (Variables|/Game/Widget/MainCanvas.MainCanvas_C|GetVideo _asmain_canvas) 0.0))