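; MyFSMManager is an actor-based finite state machine manager that cycles the game through Intro, Interaction and Ending states.
; On BeginPlay it enables input for the first player controller and enters Intro.
; SetState destroys the current state actor, then spawns the matching state class at the world origin and stores it.
; StateDone advances to the next state, looping from Ending back to Intro.
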(event EventBeginPlay
  (Input|EnableInput (Game|GetPlayerController 0))
  (CallFunction|SetState "Intro"))

(event Collision|EventActorBeginOverlap
  (params (OtherActor :type Actor%20Object%20Reference)))

(event EventTick
  (params (DeltaSeconds :type Float%20%28single-precision%29)))

(fn ConstructionScript)

(fn CreateStateActor
  (params (NewParam :type EGameState%20Enum :default "Intro"))
  (bind _returnvalue (Math|Vector|MakeVector 0.0 0.0 0.0))
  (bind _returnvalue_2 (Math|Conversions|ToTransform(Vector) _returnvalue))
  (bind _output_get (Variables|Default|SetCurrentState NewParam))
  (switch Utilities|FlowControl|Switch|SwitchonEGameState _output_get
    (:Intro
      (bind _returnvalue_3 (Game|SpawnActorfromClass "/Game/Blueprints/MyIntroState.MyIntroState_C" _returnvalue_2 "Undefined" "MultiplyWithRoot" 0 0))
      (Variables|Default|SetCurrentStateActor _returnvalue_3))
    (:Interaction
      (bind _returnvalue_4 (Game|SpawnActorfromClass "/Game/Blueprints/MyInteractionState.MyInteractionState_C" _returnvalue_2 "Undefined" "MultiplyWithRoot" 0 0))
      (Variables|Default|SetCurrentStateActor _returnvalue_4))
    (:Ending
      (bind _returnvalue_5 (Game|SpawnActorfromClass "/Game/Blueprints/MyEndingState.MyEndingState_C" _returnvalue_2 "Undefined" "MultiplyWithRoot" 0 0))
      (Variables|Default|SetCurrentStateActor _returnvalue_5))))

(fn StateDone
  (switch Utilities|FlowControl|Switch|SwitchonEGameState (Variables|Default|GetCurrentState)
    (:Intro
      (CallFunction|SetState "Interaction"))
    (:Interaction
      (CallFunction|SetState "Ending"))
    (:Ending
      (CallFunction|SetState "Intro"))))

(fn SetState
  (params (NewParam :type EGameState%20Enum :default "Intro"))
  (CallFunction|DestroyCurrentStateActor)
  (CallFunction|CreateStateActor NewParam))

(fn DestroyCurrentStateActor
  (bind _currentstateactor (Variables|Default|GetCurrentStateActor))
  (if (Utilities|IsValid _currentstateactor)
    (Actor|DestroyActor _currentstateactor)))