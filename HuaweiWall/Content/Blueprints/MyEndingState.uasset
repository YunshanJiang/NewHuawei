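; Ending-state actor that switches the Ultra Dynamic Sky to its ending condition and caches the player's MainCanvas widget.
; Tick accumulates a timer once the sky reports the sun has reached its final center.
; Pressing 1 calls StateDone on MyFSMManager.
; A timeline sequence for ending text, cine camera rotation and focal length, and growing sun and flare effects is present but disconnected, so it never runs.
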(event EventBeginPlay
  (Input|EnableInput (Game|GetPlayerController 0))
  (Development|PrintText "ending")
  (bind _asmy_character (Utilities|Casting|CastToMyCharacter (Game|GetPlayerCharacter 0)))
  (bind _output_get (Variables|Default|Setwidget (Variables|/Game/Blueprints/MyCharacter.MyCharacter_C|Getwidget _asmy_character)))
  (bind _asmain_canvas (Utilities|Casting|CastToMainCanvas _output_get))
  (bind _returnvalue (Actor|GetActorOfClass "/Game/UltraDynamicSky/Blueprints/Ultra_Dynamic_Sky.Ultra_Dynamic_Sky_C"))
  (Variables|/Game/UltraDynamicSky/Blueprints/Ultra_Dynamic_Sky.Ultra_Dynamic_Sky_C|SetCondtion _returnvalue 2))

(event Collision|EventActorBeginOverlap
  (params (OtherActor :type Actor%20Object%20Reference)))

(event EventTick
  (params (DeltaSeconds :type Float%20%28single-precision%29))
  (if (Variables|/Game/UltraDynamicSky/Blueprints/Ultra_Dynamic_Sky.Ultra_Dynamic_Sky_C|GetsunArrivedCenterFinal (stale EventBeginPlay _returnvalue))
    (bind _output_get (Variables|Default|Sett (+ (Variables|Default|Gett) DeltaSeconds)))))

(event Input|KeyboardEvents|1
  (params (Key :type Key%20Structure :default "None"))
  (:Pressed
    (bind _returnvalue (Actor|GetActorOfClass "/Game/Blueprints/MyFSMManager.MyFSMManager_C"))
    (Default|StateDone _returnvalue)))

(fn ConstructionScript)